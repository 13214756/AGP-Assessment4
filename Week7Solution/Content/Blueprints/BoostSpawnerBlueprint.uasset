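; Boost pickup actor that grants a player health, attack, defence or speed according to its Type.
; BeginPlay calls OnGenerate, then colours the skeletal mesh with a material matching the type.
; OnPickup waits briefly, then applies the boost through the player's HealthComponent, the GunBlueprint child actor's damage increase, or the character's speed boost.
; The pickup destroys itself after applying the boost.
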(event EventBeginPlay
  (Class|BoostSpawner|OnGenerate)
  (switch Utilities|FlowControl|Switch|SwitchonEBoostPickupType (Variables|Default|GetType)
    (:HEALTH
      (Rendering|Material|SetMaterial (Variables|Default|GetSkeletalMesh) 0 "/Game/Materials/GreenMaterial.GreenMaterial"))
    (:ATTACK
      (Rendering|Material|SetMaterial (Variables|Default|GetSkeletalMesh) 0 "/Game/Materials/RedMaterial.RedMaterial"))
    (:DEFENCE
      (Rendering|Material|SetMaterial (Variables|Default|GetSkeletalMesh) 0 "/Game/Materials/BlueMaterial.BlueMaterial"))
    (:SPEED
      (Rendering|Material|SetMaterial (Variables|Default|GetSkeletalMesh) 0 "/Game/Materials/BrownMaterial.BrownMaterial"))))

(event Collision|EventActorBeginOverlap
  (params (OtherActor :type Actor%20Object%20Reference)))

(event EventTick
  (params (DeltaSeconds :type Float%20%28single-precision%29)))

(event EventOnPickup
  (params (ActorThatPickedUp :type Actor%20Object%20Reference))
  (bind _returnvalue (Actor|GetComponentbyClass ActorThatPickedUp "/Script/Engine.ChildActorComponent"))
  (bind _childactor (Variables|/Script/Engine.ChildActorComponent|GetChildActor _returnvalue))
  (Utilities|IsValid (Actor|GetComponentbyClass ActorThatPickedUp "/Script/Engine.ActorComponent")
    (:Is%20Valid
      (Utilities|IsValid ActorThatPickedUp
        (:Is%20Valid
          (Utilities|FlowControl|Delay 0.1)
          (switch Utilities|FlowControl|Switch|SwitchonEBoostPickupType (Variables|Default|GetType)
            (:HEALTH
              (Utilities|IsValid ActorThatPickedUp
                (:Is%20Valid
                  (bind _asplayer_character (Utilities|Casting|CastToPlayerCharacter ActorThatPickedUp))
                  (Class|HealthComponent|Heal (Actor|GetComponentbyClass _asplayer_character "/Script/AdvGamesProgramming.HealthComponent") (Variables|Default|GetHealth))
                  (Actor|DestroyActor))))
            (:ATTACK
              (Utilities|IsValid _childactor
                (:Is%20Valid
                  (bind _asgun_blueprint (Utilities|Casting|CastToGunBlueprint _childactor))
                  (Development|PrintString "DamageBoost")
                  (Default|DamageIncrease _asgun_blueprint (Variables|Default|GetAttack))
                  (Actor|DestroyActor))))
            (:DEFENCE
              (Utilities|IsValid ActorThatPickedUp
                (:Is%20Valid
                  (bind _asplayer_character_2 (Utilities|Casting|CastToPlayerCharacter ActorThatPickedUp))
                  (Class|HealthComponent|IncreaseDefence (Actor|GetComponentbyClass _asplayer_character_2 "/Script/AdvGamesProgramming.HealthComponent") (Variables|Default|GetDefence))
                  (Actor|DestroyActor))))
            (:SPEED
              (Utilities|IsValid ActorThatPickedUp
                (:Is%20Valid
                  (bind _asplayer_character_3 (Utilities|Casting|CastToPlayerCharacter ActorThatPickedUp))
                  (Class|PlayerCharacter|ApplySpeedBoost _asplayer_character_3 (Variables|Default|GetSpeed))
                  (Actor|DestroyActor))))))))))

(fn ConstructionScript)