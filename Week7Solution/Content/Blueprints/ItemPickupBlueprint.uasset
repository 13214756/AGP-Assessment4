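; Item pickup actor that grants a health, attack, defence or speed boost, with its mesh material colored by type.
; BeginPlay calls OnGenerate and sets the material; Tick destroys the actor after a countdown while the box is closed.
; OnPickup on a closed box enables input and opens a gate fed by the E key, with no exit logic shown.
; Otherwise it applies the boost through HealthComponent or gun/character casts, then destroys itself.
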(event EventBeginPlay
  (Class|ItemPickup|OnGenerate)
  (switch Utilities|FlowControl|Switch|SwitchonEItemPickupType (Variables|Default|GetType)
    (:HEALTH
      (Rendering|Material|SetMaterial (Variables|Default|GetSkeletalMesh) 0 "/Game/Materials/GreenMaterial.GreenMaterial"))
    (:ATTACK
      (Rendering|Material|SetMaterial (Variables|Default|GetSkeletalMesh) 0 "/Game/Materials/RedMaterial.RedMaterial"))
    (:DEFENCE
      (Rendering|Material|SetMaterial (Variables|Default|GetSkeletalMesh) 0 "/Game/Materials/BlueMaterial.BlueMaterial"))
    (:SPEED
      (Rendering|Material|SetMaterial (Variables|Default|GetSkeletalMesh) 0 "/Game/Materials/BrownMaterial.BrownMaterial"))))

(event EventTick
  (params (DeltaSeconds :type Float%20%28single-precision%29))
  (if (Variables|Default|GetbBoxClosed)
    (bind _output_get (Variables|Default|SetTimeTillAutoDelete (- (Variables|Default|GetTimeTillAutoDelete) DeltaSeconds)))
    (if (<= _output_get 0.0)
      (Actor|DestroyActor))))

(event EventOnPickup
  (params (ActorThatPickedUp :type Actor%20Object%20Reference))
  (bind _returnvalue (Actor|GetComponentbyClass ActorThatPickedUp "/Script/AdvGamesProgramming.HealthComponent"))
  (Utilities|IsValid (Actor|GetComponentbyClass ActorThatPickedUp "/Script/Engine.ActorComponent")
    (:Is%20Valid
      (if (Variables|Default|GetbBoxClosed)
        (bind _asplayer_controller (Utilities|Casting|CastToPlayerController ActorThatPickedUp))
        (Input|EnableInput _asplayer_controller)
        (Utilities|FlowControl|Gate true) ; enters at Open
        (else
          (switch Utilities|FlowControl|Switch|SwitchonEItemPickupType (Variables|Default|GetType)
            (:HEALTH
              (Class|HealthComponent|Heal _returnvalue (Variables|Default|GetHealth))
              (Actor|DestroyActor))
            (:ATTACK
              (bind _asgun_blueprint (Utilities|Casting|CastToGunBlueprint ActorThatPickedUp))
              (Default|DamageIncrease _asgun_blueprint (Variables|Default|GetAttack))
              (Actor|DestroyActor))
            (:DEFENCE
              (Class|HealthComponent|IncreaseDefence _returnvalue (Variables|Default|GetDefence))
              (Actor|DestroyActor))
            (:SPEED
              (bind _asplayer_character (Utilities|Casting|CastToPlayerCharacter ActorThatPickedUp))
              (Class|PlayerCharacter|ApplySpeedBoost _asplayer_character (Variables|Default|GetSpeed))
              (Actor|DestroyActor))))))))

(event Input|KeyboardEvents|E
  (params (Key :type Key%20Structure :default "None"))
  (:Pressed
    (Utilities|FlowControl|Gate true)))

(fn ConstructionScript)